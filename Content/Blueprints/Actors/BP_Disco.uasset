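; BP_Disco is a disco light actor that endlessly flickers a PointLight with random colours and rotations.
; From BeginPlay, each cycle toggles visibility, waits a random delay between MinDelay and MaxDelay, sets a random colour and toggles visibility again.
; The ChangeRot timeline then lerps from the current world rotation toward a random rotator, and its finish calls FlickerRandomColor to restart the cycle.
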(event `self.ReceiveBeginPlay`
  (bind _pointlight (`self.PointLight`))
  (`SceneComponent.ToggleVisibility` _pointlight false :!label _label)
  (`KismetSystemLibrary.RetriggerableDelay` (`KismetMathLibrary.RandomFloatInRange` (`self.MinDelay`) (`self.MaxDelay`)))
  (`LightComponent.SetLightColor` _pointlight (`KismetMathLibrary.MakeColor` (`KismetMathLibrary.RandomFloat`) (`KismetMathLibrary.RandomFloat`) (`KismetMathLibrary.RandomFloat`)) true)
  (`SceneComponent.ToggleVisibility` _pointlight false)
  (bind _output_get (set `self.RandomRotate` (`KismetMathLibrary.RandomRotator` true)))
  (bind (_direction _changedirection) (`Timeline|ChangeRot` :!via `PlayFromStart`)
    (:`Update`
      (`SceneComponent.K2_SetWorldRotation` (`self.PointLight`) (`KismetMathLibrary.RLerp` (`SceneComponent.K2_GetComponentRotation` (`self.PointLight`)) _output_get _changedirection true) false false))
    (:`Finished`
      (`self.FlickerRandomColor`))))

(event `FlickerRandomColor`
  (goto _label))

(fn `UserConstructionScript`)