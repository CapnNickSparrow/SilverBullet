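; Tank pawn that toggles between an overview camera (CameraM) and its own Camera, gating movement and turret shooting.
; BeginPlay starts on CameraM with movement off and gravity enabled on both meshes.
; Each Start call caches transforms, then a FlipFlop runs a timeline blending CameraM to Camera or back to the Ref transform.
; Arrival enables MayMove and BP_PawnTurret shooting; the return disables both on every timeline update.
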(event `GetInfo`
  (set `self.Cam_Loc` (`SceneComponent.K2_GetComponentToWorld` (`self.Camera`)))
  (set `self.CCam_Loc` (`SceneComponent.K2_GetComponentToWorld` (`self.CameraM`)))
  (set `self.Ref_Loc` (`SceneComponent.K2_GetComponentToWorld` (`self.Ref`))))

(event `self.ReceiveBeginPlay`
  (set `self.MayMove` false)
  (`ActorComponent.SetActive` (`self.CameraM`) true false)
  (`ActorComponent.SetActive` (`self.Camera`) false false)
  (`PrimitiveComponent.SetEnableGravity` (`self.BaseMesh`) true)
  (`PrimitiveComponent.SetEnableGravity` (`self.TurretMesh`) true))

(event `Start`
  (`self.GetInfo`)
  (`/Engine/EditorBlueprintResources/StandardMacros.FlipFlop`
    (:`A`
      (bind (_direction _changecamera) (`Timeline|ChangeCamera` :!via `PlayFromStart`)
        (:`Update`
          (`SceneComponent.K2_SetWorldTransform` (`self.CameraM`) (`KismetMathLibrary.TLerp` (`self.CCam_Loc`) (`self.Cam_Loc`) _changecamera) false false))
        (:`Finished`
          (`ActorComponent.SetActive` (`self.Camera`) true false)
          (`ActorComponent.SetActive` (`self.CameraM`) false false)
          (set `self.MayMove` true)
          (bind _returnvalue (`GameplayStatics.GetActorOfClass` "/Game/Blueprints/Pawns/BP_PawnTurret.BP_PawnTurret_C"))
          (`/Game/Blueprints/Pawns/BP_PawnTurret.MayShoot` _returnvalue))))
    (:`B`
      (bind (_direction_2 _changecamera_2) (`Timeline|ChangeCam` :!via `ReverseFromEnd`)
        (:`Update`
          (`SceneComponent.K2_SetWorldTransform` (`self.CameraM`) (`KismetMathLibrary.TLerp` (`self.Ref_Loc`) (`self.CCam_Loc`) _changecamera_2) false false)
          (`ActorComponent.SetActive` (`self.CameraM`) true false)
          (`ActorComponent.SetActive` (`self.Camera`) false false)
          (set `self.MayMove` false)
          (bind _returnvalue_2 (`GameplayStatics.GetActorOfClass` "/Game/Blueprints/Pawns/BP_PawnTurret.BP_PawnTurret_C"))
          (`/Game/Blueprints/Pawns/BP_PawnTurret.StopShoot` _returnvalue_2))))))

(fn `UserConstructionScript`)